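; Test HUD Blueprint that provides drag-rectangle selection of CharacterUnit actors.
; BeginPlay creates the WB_HUD widget, adds it to the viewport and keeps a reference to it.
; While the widget's IsSelected check passes, DrawHUD runs GetActorsInSelectionRectangle between the widget's start and end positions.
; UpdateSelectedActors gathers the hits into a local Set and hands it back to the widget.
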(event EventBeginPlay
  (bind _returnvalue (UserInterface|CreateWidget "/Game/UserInterface/WB_HUD.WB_HUD_C"))
  (UserInterface|Viewport|AddtoViewport _returnvalue 0)
  (Variables|Default|SetWB_HUD _returnvalue))

(event Collision|EventActorBeginOverlap
  (params (OtherActor :type Actor%20Object%20Reference)))

(event EventTick
  (params (DeltaSeconds :type Float%20%28single-precision%29)))

(event EventDrawHUD
  (params (SizeX :type Integer) (SizeY :type Integer))
  (bind _wb_hud (Variables|Default|GetWB_HUD)
    (:then
      (Variables|/Game/UserInterface/WB_HUD.WB_HUD_C|GetIsSelected _wb_hud
        (:then
          (CallFunction|UpdateSelectedActors _wb_hud (Class|HUD|GetActorsinSelectionRectangle "/Script/Strategy.CharacterUnit" (Variables|/Game/UserInterface/WB_HUD.WB_HUD_C|GetPositionStart _wb_hud) (Variables|/Game/UserInterface/WB_HUD.WB_HUD_C|GetPositionEnd _wb_hud) true false)))
        (:else)))
    (:else)))

(fn ConstructionScript)

(fn UpdateSelectedActors
  (params (WB%20HUD :type WB%20HUD%20Object%20Reference) (NewItems :type Array%20of%20Actor%20Object%20References))
  (bind _newlocalvar (LocalVariables|GetNewLocalVar))
  (Utilities|Set|AddItems _newlocalvar NewItems)
  (Default|UpdateSelectedActors WB%20HUD _newlocalvar))