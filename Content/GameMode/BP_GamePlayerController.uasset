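; BP_GamePlayerController is a player controller that holds box-selection state, with start and end locations and a selected-actor list.
; Its only active logic is a Tick debug readout that prints the selection flags, both locations and the selected-actor count every frame.
; Nothing in this graph sets that state, BeginPlay is empty, and the screen-to-world projection nodes are left unconnected.
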(event EventBeginPlay)

(event EventTick
  (params (DeltaSeconds :type Float%20%28single-precision%29))
  (Development|PrintString (Utilities|String|ToString(Boolean) (Variables|Default|GetbIsDetectSelection)) true true "(R=0.000000,G=0.660000,B=1.000000,A=1.000000)" 0.0)
  (Development|PrintString (Utilities|String|ToString(Boolean) (Variables|Default|GetbIsSelection)) true true "(R=0.000000,G=0.660000,B=1.000000,A=1.000000)" 0.0)
  (Development|PrintString (Utilities|String|ToString(Vector) (Variables|Default|GetStartSelectionLocation)) true true "(R=0.000000,G=0.660000,B=1.000000,A=1.000000)" 0.0)
  (Development|PrintString (Utilities|String|ToString(Vector) (Variables|Default|GetEndSelectionLocation)) true true "(R=0.000000,G=0.660000,B=1.000000,A=1.000000)" 0.0)
  (Development|PrintString (Utilities|String|ToString(Integer) (Utilities|Set|Length (Variables|Default|GetSelectedActors))) true true "(R=0.000000,G=0.660000,B=1.000000,A=1.000000)" 0.0))

(fn ConstructionScript)